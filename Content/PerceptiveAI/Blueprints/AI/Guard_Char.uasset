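; Guard_Char is an AI guard character that spawns holding a weapon and ragdolls when it dies.
; On BeginPlay it spawns its WeaponClass as an owned actor, stores it and snaps it to the mesh's GripPoint socket.
; When its HealthComponent fires OnDied, the mesh switches to simulated Ragdoll physics and capsule collision turns off.
; A helper function returns the mesh's anim instance cast to ThirdPerson_AnimBP.
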(event `self.ReceiveBeginPlay`
  (bind _returnvalue (`|SpawnActorFromClass` (`self.WeaponClass`) (`KismetMathLibrary.MakeTransform` (0.0 0.0 0.0)) "AlwaysSpawn" "OverrideRootScale" self null))
  (set `self.MyWeapon` _returnvalue)
  (`self.K2_AttachToComponent` _returnvalue (`self.Mesh`) "GripPoint" "SnapToTarget" "SnapToTarget" "KeepWorld" true))

(event `self.HealthComponent.OnDied`
  (bind _mesh (`self.Mesh`))
  (`PrimitiveComponent.SetCollisionProfileName` _mesh "Ragdoll" true)
  (`SkeletalMeshComponent.SetAllBodiesSimulatePhysics` _mesh true)
  (`PrimitiveComponent.WakeAllRigidBodies` _mesh)
  (`PrimitiveComponent.SetCollisionEnabled` (`self.CapsuleComponent`) "NoCollision"))

(fn `GetAnimBlueprint`
  (returns (AnimBP :type "/Game/PerceptiveAI/Characters/Mannequin/Animations/ThirdPerson_AnimBP Object Reference"))
  (bind _asthird_person_anim_bp (cast `/Game/PerceptiveAI/Characters/Mannequin/Animations/ThirdPerson_AnimBP` (`SkeletalMeshComponent.GetAnimInstance` (`self.Mesh`))))
  (return _asthird_person_anim_bp))

(fn `UserConstructionScript`)